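; BP_AKM is a modular AKM rifle Blueprint that assembles the weapon from separate component parts.
; Its Construction Script attaches the magazine, trigger, bolt carrier and rear sight leaf to named sockets on the main static mesh component.
; All parts snap to their socket location, but only the rear sight leaf keeps its relative rotation and scale.
; The file shows no firing or animation logic.
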(fn `UserConstructionScript`
  (`SceneComponent.K2_AttachToComponent` (`self.WPN_AKM_WPN_AKM_magazine`) (`self.StaticMeshComponent`) "LowerReceiver" "SnapToTarget" "SnapToTarget" "SnapToTarget" true)
  (`SceneComponent.K2_AttachToComponent` (`self.WPN_AKM_WPN_AKM_trigger`) (`self.StaticMeshComponent`) "Trigger" "SnapToTarget" "SnapToTarget" "SnapToTarget" true)
  (`SceneComponent.K2_AttachToComponent` (`self.WPN_AKM_WPN_AKM_bolt_carrier`) (`self.StaticMeshComponent`) "EjectionPort" "SnapToTarget" "SnapToTarget" "SnapToTarget" true)
  (`SceneComponent.K2_AttachToComponent` (`self.WPN_AKM_WPN_AKM_rear_sight_leaf`) (`self.StaticMeshComponent`) "RearSight" "SnapToTarget" "KeepRelative" "KeepRelative" true))